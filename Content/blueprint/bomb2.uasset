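; Timed bomb actor tied to Player2 that explodes into four projectiles.
; On BeginPlay it waits for the BombExplode2 delay, then decrements the Bombs counter on every Player2 actor in the level.
; It then spawns a projectile at each of four spawn-point components, skipping any blocked spawn that cannot be adjusted, plays the Boom particle effect and destroys itself.
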(event EventBeginPlay
  (Utilities|FlowControl|Delay (Variables|Default|Getbomb%20explode2))
  (bind _outactors (Actor|GetAllActorsOfClass "/Game/blueprint/player2.player2_C"))
  (for _array_element _outactors
    (Math|Integer|DecrementInt (Variables|/Game/blueprint/player2.player2_C|Getbombs _array_element)))
  (Game|SpawnActorfromClass "/Game/blueprint/projectiles.projectiles_C" (Transformation|GetWorldTransform (Variables|Default|Getprojectilespawn1)) "AdjustIfPossibleButDontSpawnIfColliding" 0 0)
  (Game|SpawnActorfromClass "/Game/blueprint/projectiles.projectiles_C" (Transformation|GetWorldTransform (Variables|Default|Getprojectilespawn2)) "AdjustIfPossibleButDontSpawnIfColliding" 0 0)
  (Game|SpawnActorfromClass "/Game/blueprint/projectiles.projectiles_C" (Transformation|GetWorldTransform (Variables|Default|Getprojectilespawn3)) "AdjustIfPossibleButDontSpawnIfColliding" 0 0)
  (Game|SpawnActorfromClass "/Game/blueprint/projectiles.projectiles_C" (Transformation|GetWorldTransform (Variables|Default|Getprojectilespawn4)) "AdjustIfPossibleButDontSpawnIfColliding" 0 0)
  (Effects|SpawnEmitteratLocation "/Game/particlessystem/Boom_particlesys.Boom_particlesys" (Transformation|GetActorLocation))
  (Actor|DestroyActor))

(fn ConstructionScript)