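; Second-player Blueprint that moves a physics cube and drops bombs.
; Call2p and Call2ps share one AddForce node on the Cube, applying scaled input to both X and Y as an acceleration change.
; Call2psB spawns a Bomb2 at the cube's location and increments the Bombs count, unless that count equals Maxbombs.
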(event EventCall2ps
  (params (value :type Float%20%28single-precision%29))
  (Physics|AddForce (Variables|Default|GetCube) (Math|Vector|MakeVector (* (stale EventCall2p value) 1e+03) (* value 1e+03) 0.0) "None" true))

(event EventCall2psB
  (bind _cube (Variables|Default|GetCube))
  (bind _returnvalue (Transformation|GetWorldLocation _cube))
  (bind (_x _y _z) (Math|Vector|BreakVector _returnvalue))
  (if (!= (Variables|Default|Getbombs) (Variables|Default|Getmaxbombs))
    (Game|SpawnActorfromClass "/Game/blueprint/bomb2.bomb2_C" (Math|Conversions|ToTransform(Vector) (Math|Vector|MakeVector _x _y _z)) "Undefined" 0 0)
    (Math|Integer|IncrementInt (Variables|Default|Getbombs))))

(event EventCall2p
  (params (value :type Float%20%28single-precision%29))
  (Physics|AddForce (Variables|Default|GetCube) (Math|Vector|MakeVector (* value 1e+03) (* (stale EventCall2ps value) 1e+03) 0.0) "None" true))

(fn ConstructionScript)