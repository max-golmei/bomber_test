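; Speed pickup actor that boosts the movement speed of whichever player touches it.
; On Box overlap it checks whether the other actor is Player1 or Player2 and casts it to that class.
; It permanently adds a fixed bonus to that player's MovementSpeed variable, then destroys itself.
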(event OnComponentBeginOverlap(Box)
  (params (OverlappedComponent :type Primitive%20Component%20Object%20Reference) (OtherActor :type Actor%20Object%20Reference) (OtherComp :type Primitive%20Component%20Object%20Reference) (OtherBodyIndex :type Integer) (bFromSweep :type Boolean) (SweepResult :type Hit%20Result%20Structure%20%28by%20ref%29))
  (bind _returnvalue (Utilities|GetClass OtherActor))
  (if (== _returnvalue "/Game/blueprint/player1.player1_C")
    (bind _asplayer_1 (Utilities|Casting|CastToplayer1 OtherActor))
    (Variables|/Game/blueprint/player1.player1_C|Setmovement%20speed _asplayer_1 (+ (Variables|/Game/blueprint/player1.player1_C|Getmovement%20speed _asplayer_1) 3e+02))
    (Actor|DestroyActor :!label _label)
    (elif (== _returnvalue "/Game/blueprint/player2.player2_C")
      (bind _asplayer_2 (Utilities|Casting|CastToplayer2 OtherActor))
      (Variables|/Game/blueprint/player2.player2_C|Setmovement%20speed _asplayer_2 (+ (Variables|/Game/blueprint/player2.player2_C|Getmovement%20speed _asplayer_2) 3e+02))
      (goto _label))))

(fn ConstructionScript)