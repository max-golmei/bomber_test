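; Breakable wall actor that can drop a power-up pickup when destroyed.
; On Destroyed, a random roll spawns a Bombbooster at the Cube's world location, otherwise further rolls may spawn a Playerspeed there.
; Each check draws a fresh random number, so the Playerspeed range test is two independent rolls rather than one band, and often nothing drops.
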(event EventDestroyed
  (bind _returnvalue (Math|Random|RandomFloatinRange 0.0 1e+02))
  (bind _cube (Variables|Default|GetCube))
  (bind _returnvalue_2 (Transformation|GetWorldLocation _cube))
  (bind _returnvalue_3 (Math|Conversions|ToTransform(Vector) _returnvalue_2))
  (if (< _returnvalue 4e+01)
    (Game|SpawnActorfromClass "/Game/blueprint/bombbooster.bombbooster_C" _returnvalue_3 "Undefined" 0 0)
    (elif (and (< _returnvalue 8e+01) (> _returnvalue 5e+01))
      (Game|SpawnActorfromClass "/Game/blueprint/playerspeed.playerspeed_C" _returnvalue_3 "Undefined" 0 0))))

(fn ConstructionScript)