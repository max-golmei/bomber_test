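; Bomb actor for Player1 that detonates two seconds after spawning, in what appears to be a Bomberman-style game.
; On detonation it decrements the Bombs count on every Player1 actor, then checks the actors overlapping its sphere.
; It destroys overlapping Player1 and Player2 actors, and calls DropChance on breakable walls before destroying them.
; The bomb then destroys itself.
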(event EventBeginPlay
  (Utilities|FlowControl|Delay 2.0)
  (bind _outactors (Actor|GetAllActorsOfClass "/Game/blueprint/player1.player1_C"))
  (for _array_element _outactors
    (Math|Integer|DecrementInt (Variables|/Game/blueprint/player1.player1_C|Getbombs _array_element)))
  (bind _output_get (Variables|Default|SetNewVar_0 (Collision|GetOverlappingActors (Variables|Default|GetSphere1) 0 :!class /Script/Engine.PrimitiveComponent)))
  (for _array_element_2 _output_get
    (if (or (== (Utilities|GetClass _array_element_2) "/Game/blueprint/player2.player2_C") (== (Utilities|GetClass _array_element_2) "/Game/blueprint/player1.player1_C"))
      (Actor|DestroyActor _array_element_2)
      (elif (== (Utilities|GetClass _array_element_2) "/Game/blueprint/breakablewall.breakablewall_C")
        (bind _asbreakablewall (Utilities|Casting|CastTobreakablewall _array_element_2))
        (Default|DropChance _asbreakablewall)
        (Actor|DestroyActor _array_element_2))))
  (Actor|DestroyActor))

(fn ConstructionScript)