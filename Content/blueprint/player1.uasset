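; Player 1 Blueprint for a two-player bomb game, which also receives and relays Player 2's input.
; The forward and left axes share one AddForce on the physics Cube, driving X and Y from the same value.
; The "player1 forward/right" axes and Enter are forwarded to Player2 actors found with GetAllActorsOfClass.
; Space spawns a Bomb1 at the Cube and increments Bombs until it equals Maxbombs.
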(event EventTick
  (params (DeltaSeconds :type Float%20%28single-precision%29)))

(event Input|AxisEvents|InputAxisforward
  (params (AxisValue :type Float%20%28single-precision%29))
  ;[1 1 1] input to player 1
  (Physics|AddForce (Variables|Default|GetCube) (Math|Vector|MakeVector (* AxisValue 1e+03) (* (stale Input|AxisEvents|InputAxisleft AxisValue) 1e+03) 0.0) "None" true))

(event Input|AxisEvents|InputAxisplayer1forward
  (params (AxisValue :type Float%20%28single-precision%29))
  (bind _outactors (Actor|GetAllActorsOfClass "/Game/blueprint/player2.player2_C"))
  (Default|Call2p _outactors AxisValue))

(event Input|AxisEvents|InputAxisleft
  (params (AxisValue :type Float%20%28single-precision%29))
  ;[1 1 1] input to player 1
  (Physics|AddForce (Variables|Default|GetCube) (Math|Vector|MakeVector (* (stale Input|AxisEvents|InputAxisforward AxisValue) 1e+03) (* AxisValue 1e+03) 0.0) "None" true))

(event Input|AxisEvents|InputAxisplayer1right
  (params (AxisValue :type Float%20%28single-precision%29))
  (bind _outactors (Actor|GetAllActorsOfClass "/Game/blueprint/player2.player2_C"))
  (Default|Call2ps _outactors AxisValue))

(event Input|KeyboardEvents|SpaceBar
  (params (Key :type Key%20Structure))
  (bind _cube (Variables|Default|GetCube))
  (bind _returnvalue (Transformation|GetWorldLocation _cube))
  (bind (_x _y _z) (Math|Vector|BreakVector _returnvalue))
  (:Pressed
    (if (!= (Variables|Default|Getbombs) (Variables|Default|Getmaxbombs))
      (Game|SpawnActorfromClass "/Game/blueprint/bomb1.bomb1_C" (Math|Conversions|ToTransform(Vector) (Math|Vector|MakeVector _x _y _z)) "Undefined" 0 0)
      (Math|Integer|IncrementInt (Variables|Default|Getbombs)))))

(event Input|KeyboardEvents|Enter
  (params (Key :type Key%20Structure))
  (:Pressed
    (bind _outactors (Actor|GetAllActorsOfClass "/Game/blueprint/player2.player2_C"))
    (Default|Call2psB _outactors)))

(fn ConstructionScript)